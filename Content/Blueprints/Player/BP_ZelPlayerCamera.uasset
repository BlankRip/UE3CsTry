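; BP_ZelPlayerCamera is a player camera actor that follows a target player.
; SetTargetPlayer stores the target, makes this actor the view target of its BP_ZelPlayerController and enables Tick.
; Tick snaps the actor to the target's location each frame without sweeping, and ClearTargetPlayer drops the target and disables Tick.
; SetCameraMaxDistance sets the SpringArm's target arm length to adjust camera distance.
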(event `self.ReceiveTick`
  (params (DeltaSeconds :type "Float (single-precision)"))
  (`self.K2_SetActorLocation` (`self.K2_GetActorLocation` (`self.TargetPlayer`))))

(fn `ClearTargetPlayer`
  (set `self.TargetPlayer` null)
  (`self.SetActorTickEnabled` false))

(fn `SetCameraMaxDistance`
  (params (`Target Arm Length` :type "Float (single-precision)" :default 300.0))
  (set `SpringArmComponent.TargetArmLength` `Target Arm Length` (`self.SpringArm`)))

(fn `SetTargetPlayer`
  (params (TargetPlayer :type "/Game/Blueprints/Player/BP_ZelCharacter Object Reference"))
  (bind _output_get (set `self.TargetPlayer` TargetPlayer))
  (bind _asbp_zel_player_controller (cast `/Game/Blueprints/Player/BP_ZelPlayerController` (`Pawn.GetController` _output_get)))
  (`PlayerController.SetViewTargetWithBlend` _asbp_zel_player_controller self 0.0 "VTBlend_Linear" 0.0 false)
  (`self.SetActorTickEnabled` true))

(fn `UserConstructionScript`)