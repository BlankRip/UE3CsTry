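; Base Blueprint for usable pickups that a BP_ZelCharacter takes by interacting with them.
; StartInteraction disables collision and physics, hands the pickup and its attachment offset to the character, blocks further interaction and calls OnPickup.
; OnPickup and OnMovedUpdate are empty hooks, apparently for subclasses, with move updates gated by a flag.
; RequestUse returns true by default, and IsInteractable reports the CanInteract state.
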(event `/Game/Blueprints/InteractionSystem/InteractableWorldItem/BPI_WorldInteratable.StartInteraction`
  (params (InteractingActor :type "Actor Object Reference"))
  (bind _asbp_zel_character (cast `/Game/Blueprints/Player/BP_ZelCharacter` InteractingActor))
  (`self.SetActorEnableCollision` false)
  (`PrimitiveComponent.SetSimulatePhysics` (`self.SimulatedPhysicsRoot`) false)
  (`/Game/Blueprints/Player/BP_ZelCharacter.SetUsablePickup` _asbp_zel_character self (`self.CharacterAttachmentOffset`))
  (set `self.CanInteract` false)
  (`self.OnPickup` _asbp_zel_character))

(fn `IsInteractable`
  (returns (CanInteract :type Boolean))
  (return (`self.CanInteract`)))

(fn `OnMovedUpdate`)

(fn `OnPickup`
  (params (PickUpOwner :type "Actor Object Reference")))

(fn `RequestOnMovedUpdate`
  (if (`self.ShouldRunOnMoveUpdate`)
    (`self.OnMovedUpdate`)))

(fn `RequestUse`
  (returns (AllUsesDepleted :type Boolean))
  (return true))

(fn `UserConstructionScript`)