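; Base actor for interactable pickups that a character can carry and use.
; On interaction by an actor implementing BPI_PickupUser, it disables collision and physics, passes itself and an attachment offset to that actor, stops being interactable and calls OnPickup.
; OnPickup and OnMovedUpdate are empty hooks, the latter gated by ShouldRunOnMoveUpdate, while RequestUse returns true by default.
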(event `/Game/Blueprints/InteractionSystem/InteractableWorldItem/BPI_WorldInteratable.StartInteraction`
  (params (InteractingActor :type "Actor Object Reference"))
  (if (`KismetSystemLibrary.DoesImplementInterface` InteractingActor "/Game/Blueprints/LevelObjects/Interactables/PickUps/BPI_PickupUser.BPI_PickupUser_C")
    (`self.SetActorEnableCollision` false)
    (`PrimitiveComponent.SetSimulatePhysics` (`self.SimulatedPhysicsRoot`) false)
    (message `/Game/Blueprints/LevelObjects/Interactables/PickUps/BPI_PickupUser.SetUsablePickup` InteractingActor self (`self.CharacterAttachmentOffset`))
    (set `self.CanInteract` false)
    (`self.OnPickup` InteractingActor)))

(fn `IsInteractable`
  (returns (CanInteract :type Boolean))
  (return (`self.CanInteract`)))

(fn `OnMovedUpdate`)

(fn `OnPickup`
  (params (PickUpOwner :type "Actor Object Reference")))

(fn `RequestOnMovedUpdate`
  (if (`self.ShouldRunOnMoveUpdate`)
    (`self.OnMovedUpdate`)))

(fn `RequestUse`
  (returns (AllUsesDepleted :type Boolean))
  (return true))

(fn `UserConstructionScript`)