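; BP_Bomb is a throwable bomb pickup that shows a highlight as its ready-to-interact cue.
; RequestUse calls the parent logic, detaches the bomb, re-enables collision and physics, then launches it forward with a velocity-change impulse scaled by LaunchVelocity.
; A physics root hit destroys the actor if CanInteract is false; no explosion or damage is implemented here.
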(event `self.ReceiveBeginPlay`
  (`parent.ReceiveBeginPlay`))

(event `/Game/Blueprints/InteractionSystem/InteractableWorldItem/BPI_WorldInteratable.ShowReadyToInteractCue`
  (`SceneComponent.SetHiddenInGame` (`self.Highlight`) false false))

(event `/Game/Blueprints/InteractionSystem/InteractableWorldItem/BPI_WorldInteratable.HideReadyToInteractCue`
  (`SceneComponent.SetHiddenInGame` (`self.Highlight`) true false))

(event `self.SimulatedPhysicsRoot.OnComponentHit`
  (params (HitComponent :type "PrimitiveComponent Object Reference") (OtherActor :type "Actor Object Reference") (OtherComp :type "PrimitiveComponent Object Reference") (NormalImpulse :type "Vector Structure") (Hit :type "HitResult Structure (by ref)"))
  (if (not (`self.CanInteract`))
    (`self.K2_DestroyActor`)))

(fn `RequestUse`
  (returns (AllUsesDepleted :type Boolean))
  (bind _simulatedphysicsroot (`self.SimulatedPhysicsRoot`))
  (bind _allusesdepleted (`parent.RequestUse`))
  (`self.K2_DetachFromActor` "KeepWorld" "KeepWorld" "KeepWorld")
  (`self.SetActorEnableCollision` true)
  (`PrimitiveComponent.SetSimulatePhysics` _simulatedphysicsroot true)
  (`PrimitiveComponent.AddImpulse` _simulatedphysicsroot (* (`self.GetActorForwardVector`) (`self.LaunchVelocity`)) "None" true)
  (return _allusesdepleted))

(fn `UserConstructionScript`
  (`parent.UserConstructionScript`))